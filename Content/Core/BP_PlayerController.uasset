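; Player controller that handles the in-game text chat: forwarding messages and toggling the chat window.
; SendToPlayerController_GS relays a sender and message to BP_GameState through OnMessageSendToGSEvent.
; The Chat input action uses the widget switcher index in the HUD's chat window to decide whether to show or hide it.
; Showing chat enables the cursor, focuses the text box and disables pawn input; hiding restores game-only control.
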(event `SendToPlayerController_GS`
  (params (Sender :type String) (Message :type String))
  (bind _asbp_game_state (cast `/Game/Core/BP_GameState` (`GameplayStatics.GetGameState`)))
  (`/Game/Core/BP_GameState.OnMessageSendToGS_Event` _asbp_game_state Sender Message))

(event `InputAction|Chat`
  (params (Key :type "Key Structure"))
  (:`Pressed`
    (bind _asbp_hud (cast `/Game/Core/BP_HUD` (`self.GetHUD`)))
    (bind _wbp_chatwindow (`/Game/UI/WBP_ChatOnScreen.WBP_ChatWindow` (`/Game/Core/BP_HUD.Chat On Screen` _asbp_hud)))
    (if (== (`WidgetSwitcher.ActiveWidgetIndex` (`/Game/UI/WBP_ChatWindow.WidgetSwitcher` _wbp_chatwindow)) 0)
      (`/Game/UI/WBP_ChatWindow.Show Chat` _wbp_chatwindow)
      (set `self.bShowMouseCursor` true)
      (`WidgetBlueprintLibrary.SetInputMode_GameAndUIEx` self (`/Game/UI/WBP_ChatWindow.EnteredTextBox` _wbp_chatwindow))
      (`self.DisableInput` (`self.K2_GetPawn`) self)
      (else
        (`/Game/UI/WBP_ChatWindow.Hide Chat` _wbp_chatwindow)
        (set `self.bShowMouseCursor` false)
        (`WidgetBlueprintLibrary.SetInputMode_GameOnly` self)
        (`self.EnableInput` (`self.K2_GetPawn`) self)))))

(fn `UserConstructionScript`)